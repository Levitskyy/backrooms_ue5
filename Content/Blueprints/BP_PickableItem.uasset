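; Base pickable item actor that simulates physics in the world and can be picked up through interaction, carried and dropped.
; Pickup and Drop set AttachedParent, whose RepNotify either snaps the item to the owner's camera with physics and collision off, or detaches it and restores both.
; Other RepNotifies toggle mesh visibility and hand freshly spawned items to the matching local first-person character's slot.
; UseItemEvent is an empty hook.
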(event `self.ReceiveBeginPlay`
  (`parent.ReceiveBeginPlay`)
  (`PrimitiveComponent.SetSimulatePhysics` (`self.Mesh`) true))

(event `self.ReceiveActorBeginOverlap`
  (params (OtherActor :type "Actor Object Reference"))
  (`parent.ReceiveActorBeginOverlap` OtherActor))

(event `/Game/Blueprints/Interfaces/BPI_Interactable.Interact`
  (params (Invoker :type "Actor Object Reference"))
  (`self.Pickup` Invoker))

(event `AttachedItem`
  (params (Owner :type "Actor Object Reference"))
  (bind _mesh (`self.Mesh`))
  ;[1 1 1] Pick up this item
  (`PrimitiveComponent.SetSimulatePhysics` _mesh false)
  (`PrimitiveComponent.SetCollisionEnabled` _mesh "NoCollision")
  (`self.K2_AttachToComponent` (`self.GetComponentByClass` Owner "/Script/Engine.CameraComponent") "None" "SnapToTarget" "SnapToTarget" "KeepRelative" false)
  (`KismetSystemLibrary.MoveComponentTo` _mesh (100.0 30.0 -30.0) (struct) false false 0.0))

(event `/Game/Blueprints/Interfaces/BPI_Pickable.Pickup`
  (params (Owner :type "Actor Object Reference"))
  ;[1 1 1] Pick up this item
  (set `self.AttachedParent` Owner))

(event `/Game/Blueprints/Interfaces/BPI_Pickable.Drop`
  (params (Owner :type "Actor Object Reference"))
  ;[1 1 1] Drop this item
  (set `self.AttachedParent` null))

(event `DetachedItem`
  (params (Owner :type "Actor Object Reference"))
  (bind _mesh (`self.Mesh`))
  ;[1 1 1] Drop this item
  (`self.K2_DetachFromActor` "KeepWorld" "KeepWorld")
  (`PrimitiveComponent.SetCollisionEnabled` _mesh "QueryAndPhysics")
  (`PrimitiveComponent.SetSimulatePhysics` _mesh true)
  (`SceneComponent.SetVisibility` _mesh true false))

(event `UseItemEvent`)

(fn `OnRep_AttachedParent`
  (bind _attachedparent (`self.AttachedParent`))
  (if (`KismetSystemLibrary.IsValid` _attachedparent)
    (`self.AttachedItem` _attachedparent)
    (else
      (`self.DetachedItem` null))))

(fn `OnRep_isActive?`
  (`SceneComponent.SetVisibility` (`self.Mesh`) (`self.isActive?`) false))

(fn `OnRep_SpawnInit`
  (bind (_parent _slotindex) (break `/Game/Blueprints/PickableItems/Structs/PickupInitializeMeta` (`self.SpawnInit`)))
  (bind _asbp_first_person_character (cast `/Game/FirstPerson/Blueprints/BP_FirstPersonCharacter` (`GameplayStatics.GetPlayerCharacter` 0)))
  (if (== _asbp_first_person_character _parent)
    (`/Game/FirstPerson/Blueprints/BP_FirstPersonCharacter.PickupItemAfterSpawn` _asbp_first_person_character self _slotindex)))

(fn `SetAttachedParent`
  (params (Parent :type "Actor Object Reference"))
  (set `self.AttachedParent` Parent))

(fn `UserConstructionScript`
  (`parent.UserConstructionScript`))