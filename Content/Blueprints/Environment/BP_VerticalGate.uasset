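; Vertical gate actor that sinks its mesh when Opened is true and raises it back when false.
; BeginPlay records the actor's starting Z and fixes the travel distance in GateHeight.
; Tick moves GateMesh at Speed scaled by delta time, tracking CurrentHeight separately to stop at either end, without clamping the final step.
; Nothing in this Blueprint sets Opened.
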(event `self.ReceiveBeginPlay`
  (bind _output_get (set `self.StartHeight` (.z (.location (`self.GetTransform`)))))
  (set `self.CurrentHeight` _output_get)
  (set `self.GateHeight` 400.0))

(event `self.ReceiveTick`
  (params (DeltaSeconds :type "Float (single-precision)"))
  (bind (_returnvalue_x _returnvalue_y _returnvalue_z) (`KismetMathLibrary.BreakVector` (`SceneComponent.GetSocketLocation` (`self.GateMesh`) "None")))
  (bind _returnvalue (* (`self.Speed`) DeltaSeconds -1.0))
  (bind _returnvalue_2 (* DeltaSeconds (`self.Speed`)))
  (if (`self.Opened?`)
    (if (< (- (`self.StartHeight`) (`self.CurrentHeight`)) (`self.GateHeight`))
      (`SceneComponent.K2_SetWorldLocation` (`self.GateMesh`) (`KismetMathLibrary.MakeVector` _returnvalue_x _returnvalue_y (+ _returnvalue _returnvalue_z)) false false)
      (set `self.CurrentHeight` (+ (`self.CurrentHeight`) _returnvalue)))
    (elif (>= (- (`self.StartHeight`) (`self.CurrentHeight`)) 0.0)
      (`SceneComponent.K2_SetWorldLocation` (`self.GateMesh`) (`KismetMathLibrary.MakeVector` _returnvalue_x _returnvalue_y (+ _returnvalue_z _returnvalue_2)) false false)
      (set `self.CurrentHeight` (+ (`self.CurrentHeight`) _returnvalue_2)))))

(fn `UserConstructionScript`)