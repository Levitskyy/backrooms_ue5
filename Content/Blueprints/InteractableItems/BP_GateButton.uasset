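; BP_GateButton is an interactable button that opens and closes a connected gate.
; Its Interact event calls ChangeState on ConnectedGate with the inverse of the gate's Opened value, so each use toggles it.
; GetDisplayText always returns "Open Gate", regardless of the gate's current state.
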(event `/Game/Blueprints/BP_Item.Interact`
  (params (Invoker :type "Actor Object Reference"))
  (bind _connectedgate (`self.ConnectedGate`))
  (`/Game/Blueprints/Environment/BP_VerticalGate.ChangeState` _connectedgate (not (`/Game/Blueprints/Environment/BP_VerticalGate.Opened?` _connectedgate))))

(fn `GetDisplayText`
  (returns (DisplayText :type Text))
  (return "Open Gate"))

(fn `UserConstructionScript`
  (`parent.UserConstructionScript`))