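; BP_WinButton is an interactable win button that ends the game and returns to the main menu.
; On BeginPlay the server destroys it with a 90% chance, so it only occasionally remains in the level.
; Interacting sets HasWon, whose OnRep handler is empty, then after a short delay LeaveToMenu opens the MainMenu level and switches to UI-only input with the cursor shown.
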(event `self.ReceiveBeginPlay`
  (if (`KismetSystemLibrary.IsServer`)
    (if (< (`KismetMathLibrary.RandomFloat`) 0.9)
      (`self.DeleteButton`))))

(event `DeleteButton`
  (`self.K2_DestroyActor`))

(event `/Game/Blueprints/Interfaces/BPI_Interactable.Interact`
  (params (Invoker :type "Actor Object Reference"))
  (set `self.HasWon` true)
  (`KismetSystemLibrary.Delay` 5.0)
  (`self.LeaveToMenu`))

(fn `LeaveToMenu`
  (bind _returnvalue (`GameplayStatics.GetPlayerController` 0))
  (`GameplayStatics.OpenLevel` "MainMenu")
  (set `PlayerController.bShowMouseCursor` true _returnvalue)
  (`WidgetBlueprintLibrary.SetInputMode_UIOnlyEx` _returnvalue null "LockInFullscreen" true))

(fn `OnRep_HasWon`)

(fn `UserConstructionScript`)