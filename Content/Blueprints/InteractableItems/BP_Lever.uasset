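; Interactable lever, labeled "Open Gate", that controls a connected gate.
; Interact toggles the replicated LeverUp flag, whose RepNotify calls ChangeState to play or reverse the UpDown timeline.
; The timeline lerps the lever's roll between 0 and 60 degrees, and on finish copies LeverUp to the gate's Opened flag.
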(event `self.ReceiveBeginPlay`)

(event `/Game/Blueprints/BP_Item.Interact`
  (params (Invoker :type "Actor Object Reference"))
  (set `self.LeverUp?` (not (`self.LeverUp?`))))

(event `ChangeState`
  (bind (_returnvalue_roll _returnvalue_pitch _returnvalue_yaw) (`KismetMathLibrary.BreakRotator` (`self.K2_GetActorRotation`)))
  (if (`self.LeverUp?`)
    (bind (_direction _leveruptrack) (`Timeline|Up/Down` :!label _label)
      (:`Update`
        (`self.K2_SetActorRotation` (`KismetMathLibrary.MakeRotator` (`KismetMathLibrary.Lerp` 0.0 60.0 _leveruptrack) _returnvalue_pitch _returnvalue_yaw)))
      (:`Finished`
        (set `/Game/Blueprints/Environment/BP_VerticalGate.Opened?` (`self.LeverUp?`) (`self.ConnectedGate`))))
    (else
      (goto _label :!via `Reverse`))))

(fn `GetDisplayText`
  (returns (DisplayText :type Text))
  (return "Open Gate"))

(fn `OnRep_LeverUp?`
  (`self.ChangeState`))

(fn `UserConstructionScript`)