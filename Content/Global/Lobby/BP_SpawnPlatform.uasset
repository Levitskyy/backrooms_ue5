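; Lobby spawn platform actor that displays a first-person character for an assigned player controller.
; SpawnCharacter stores the controller, destroys any current character and spawns a BP_FirstPersonCharacter at PlayerSpawnPoint, keeping it as CurrChar.
; DeleteCharacter clears the controller and destroys that character.
; On BeginPlay the platform gives its light a random color, with each channel clamped to a mid range.
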(event `SpawnCharacter`
  (params (PC :type "PlayerController Object Reference"))
  (bind _currchar (`self.CurrChar`))
  ;[1 1 1] Spawning character on a platform
  (set `self.PC` PC)
  (`/Engine/EditorBlueprintResources/StandardMacros.IsValid` _currchar
    (:`Is Valid`
      (`self.K2_DestroyActor` _currchar))
    (:`Is Not Valid`
      _))
  (bind _returnvalue (`|SpawnActorFromClass` "/Game/FirstPerson/Blueprints/BP_FirstPersonCharacter.BP_FirstPersonCharacter_C" (`SceneComponent.K2_GetComponentToWorld` (`self.PlayerSpawnPoint`)) "Undefined" "MultiplyWithRoot" null null))
  (set `self.CurrChar` _returnvalue))

(event `DeleteCharacter`
  (bind _currchar (`self.CurrChar`))
  ;[1 1 1] Deleting character
  (set `self.PC` null)
  (`/Engine/EditorBlueprintResources/StandardMacros.IsValid` _currchar
    (:`Is Valid`
      (`self.K2_DestroyActor` _currchar)
      (set `self.CurrChar` null))))

(event `self.ReceiveBeginPlay`
  ;[1 1 1] Set random light color
  (bind _output_get (set `self.PlatformColor` (`KismetMathLibrary.MakeColor` (`KismetMathLibrary.FClamp` (`KismetMathLibrary.RandomFloat`) 0.3 0.8) (`KismetMathLibrary.FClamp` (`KismetMathLibrary.RandomFloat`) 0.3 0.8) (`KismetMathLibrary.FClamp` (`KismetMathLibrary.RandomFloat`) 0.3 0.8))))
  (`LightComponent.SetLightColor` (`self.Light`) _output_get true))

(fn `UserConstructionScript`)