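; BP_Enemy1 is an AI enemy pawn that chases players and kills them on contact.
; PawnSensing sets a seen flag, never cleared here, and passes the sighted pawn to FollowPlayer, which runs AIMoveTo toward it.
; On hitting a BP_FirstPersonCharacter, the server sets that character's IsDead and destroys the enemy itself.
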(event `self.ReceiveHit`
  (params (MyComp :type "PrimitiveComponent Object Reference") (Other :type "Actor Object Reference") (OtherComp :type "PrimitiveComponent Object Reference") (bSelfMoved :type Boolean) (HitLocation :type "Vector Structure") (HitNormal :type "Vector Structure") (NormalImpulse :type "Vector Structure") (Hit :type "HitResult Structure (by ref)"))
  (bind _asbp_first_person_character (cast `/Game/FirstPerson/Blueprints/BP_FirstPersonCharacter` Other))
  (if (`KismetSystemLibrary.IsServer`)
    (set `/Game/FirstPerson/Blueprints/BP_FirstPersonCharacter.IsDead` true _asbp_first_person_character)
    (`self.K2_DestroyActor` (`ActorComponent.GetOwner` MyComp))))

(event `self.PawnSensing.OnSeePawn`
  (params (Pawn :type "Pawn Object Reference"))
  (set `self.isSeingPlayer` true)
  (`self.FollowPlayer` Pawn))

(event `FollowPlayer`
  (params (Target :type "Actor Object Reference"))
  (if (`self.isSeingPlayer`)
    (`|AIMoveTo` self (0.0 0.0 0.0) Target 0.0)))

(fn `UserConstructionScript`)