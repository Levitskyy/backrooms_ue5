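; Level generator actor that builds the floor at runtime by spawning random rooms on a grid as the player moves.
; Each Tick, GetIdByPosition flattens the player's X/Y cell into one ID using RoomSize and LevelSize.
; If SpawnedRooms lacks that ID, SpawnRoom places a random RoomTypes class at the grid position minus a fixed X/Y offset.
; It then records the ID computed from that offset position, not the player's.
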(event `self.ReceiveBeginPlay`)

(event `self.ReceiveTick`
  (params (DeltaSeconds :type "Float (single-precision)"))
  (bind _roomsize (`self.RoomSize`))
  (bind (_id _currentplayerposition) (`self.GetIdByPosition` (0.0 0.0 0.0) true))
  (if (not (`KismetArrayLibrary.Array_Contains` (`self.SpawnedRooms`) _id))
    (`self.SpawnRoom` (`KismetMathLibrary.MakeVector` (- (* (`.ReturnValue` (`KismetMathLibrary.FMod` (.x _currentplayerposition) _roomsize)) _roomsize) 1000.0) (- (* (`.ReturnValue` (`KismetMathLibrary.FMod` (.y _currentplayerposition) _roomsize)) _roomsize) 1000.0)))))

(fn `GetIdByPosition`
  (params (Position :type "Vector Structure") (UseCurrentPlayerPosition :type Boolean))
  (returns (id :type Integer) (CurrentPlayerPosition :type "Vector Structure"))
  (bind _roomsize (`self.RoomSize`))
  (bind _roomsize_2 (`self.RoomSize`))
  (bind _returnvalue (`self.K2_GetActorLocation` (`GameplayStatics.GetPlayerCharacter` 0)))
  (if UseCurrentPlayerPosition
    (return (+ (* (`.ReturnValue` (`KismetMathLibrary.FMod` (.x _returnvalue) _roomsize)) (`self.LevelSize`)) (`.ReturnValue` (`KismetMathLibrary.FMod` (.y _returnvalue) _roomsize))) _returnvalue)
    (else
      (return (+ (* (`.ReturnValue` (`KismetMathLibrary.FMod` (.x Position) _roomsize_2)) (`self.LevelSize`)) (`.ReturnValue` (`KismetMathLibrary.FMod` (.y Position) _roomsize_2))) (0.0 0.0 0.0)))))

(fn `SpawnRoom`
  (params (`Room position` :type "Vector Structure"))
  (`|SpawnActorFromClass` (`KismetArrayLibrary.Array_Random` (`self.RoomTypes`)) (`KismetMathLibrary.Conv_VectorToTransform` `Room position`) "AdjustIfPossibleButAlwaysSpawn" "MultiplyWithRoot" null null)
  (bind _id (`self.GetIdByPosition` `Room position`))
  (`KismetArrayLibrary.Array_Add` (`self.SpawnedRooms`) _id))

(fn `UserConstructionScript`)