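; BP_TPRoomInGame is a room assembly that bundles two vertical gates, two levers, an old computer and a key loader as child actors.
; On BeginPlay it casts each child actor to its Blueprint class and caches the references.
; It then links each lever to its matching gate and the computer to the key loader, leaving any interaction logic to those Blueprints.
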(event `self.ReceiveBeginPlay`
  (`|ExecutionSequence`
    (:`then_0`
      (bind _asbp_vertical_gate (cast `/Game/Blueprints/Environment/BP_VerticalGate` (`ChildActorComponent.ChildActor` (`self.BP_VerticalGate1`))))
      (set `self.Gate1` _asbp_vertical_gate)
      (bind _asbp_vertical_gate_2 (cast `/Game/Blueprints/Environment/BP_VerticalGate` (`ChildActorComponent.ChildActor` (`self.BP_VerticalGate2`))))
      (set `self.Gate2` _asbp_vertical_gate_2)
      (bind _asbp_lever (cast `/Game/Blueprints/InteractableItems/BP_Lever` (`ChildActorComponent.ChildActor` (`self.BP_Lever1`))))
      (set `self.Lever1` _asbp_lever)
      (bind _asbp_lever_2 (cast `/Game/Blueprints/InteractableItems/BP_Lever` (`ChildActorComponent.ChildActor` (`self.BP_Lever2`))))
      (set `self.Lever2` _asbp_lever_2)
      (bind _asbp_old_computer (cast `/Game/Lobby/Blueprints/Interactable/BP_OldComputer` (`ChildActorComponent.ChildActor` (`self.BP_OldComputer`))))
      (set `self.Computer` _asbp_old_computer)
      (bind _asbp_key_loader (cast `/Game/Lobby/Blueprints/Interactable/BP_KeyLoader` (`ChildActorComponent.ChildActor` (`self.BP_KeyLoader`))))
      (set `self.KeyLoader` _asbp_key_loader))
    (:`then_1`
      (set `/Game/Blueprints/InteractableItems/BP_Lever.ConnectedGate` (`self.Gate1`) (`self.Lever1`))
      (set `/Game/Blueprints/InteractableItems/BP_Lever.ConnectedGate` (`self.Gate2`) (`self.Lever2`))
      (set `/Game/Lobby/Blueprints/Interactable/BP_OldComputer.ConnectedKeyLoader` (`self.KeyLoader`) (`self.Computer`)))))

(fn `UserConstructionScript`)