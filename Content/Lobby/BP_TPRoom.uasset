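; BP_TPRoom is a lobby room actor that pairs two levers with two vertical gates.
; On BeginPlay it casts its four child actors to BP_VerticalGate and BP_Lever and caches them, then sets each lever's ConnectedGate to its matching gate.
; It holds no gate or lever behavior of its own, only this runtime wiring.
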(event `self.ReceiveBeginPlay`
  (`|ExecutionSequence`
    (:`then_0`
      (bind _asbp_vertical_gate (cast `/Game/Blueprints/Environment/BP_VerticalGate` (`ChildActorComponent.ChildActor` (`self.BP_VerticalGate1`))))
      (set `self.Gate1` _asbp_vertical_gate)
      (bind _asbp_vertical_gate_2 (cast `/Game/Blueprints/Environment/BP_VerticalGate` (`ChildActorComponent.ChildActor` (`self.BP_VerticalGate2`))))
      (set `self.Gate2` _asbp_vertical_gate_2)
      (bind _asbp_lever (cast `/Game/Blueprints/InteractableItems/BP_Lever` (`ChildActorComponent.ChildActor` (`self.BP_Lever1`))))
      (set `self.Lever1` _asbp_lever)
      (bind _asbp_lever_2 (cast `/Game/Blueprints/InteractableItems/BP_Lever` (`ChildActorComponent.ChildActor` (`self.BP_Lever2`))))
      (set `self.Lever2` _asbp_lever_2))
    (:`then_1`
      (set `/Game/Blueprints/InteractableItems/BP_Lever.ConnectedGate` (`self.Gate1`) (`self.Lever1`))
      (set `/Game/Blueprints/InteractableItems/BP_Lever.ConnectedGate` (`self.Gate2`) (`self.Lever2`)))))

(fn `UserConstructionScript`)